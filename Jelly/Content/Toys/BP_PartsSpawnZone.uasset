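; Spawn zone that periodically creates random toy parts (BP_ToyMember) for the FunFactory game mode.
; Tick accumulates time and calls SpawnPart every MAXTIME, which spawns at the Box center with random yaw when Spawn is set.
; Toy type is random up to the game mode's DifficultyLevel, and part is random within the enum.
; ObtainMesh supplies the Init mesh from separate random rolls, so it can mismatch the spawned Type and Part.
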(event `self.ReceiveBeginPlay`)

(event `self.ReceiveActorBeginOverlap`
  (params (OtherActor :type "Actor Object Reference")))

(event `self.ReceiveTick`
  (params (DeltaSeconds :type "Float (single-precision)"))
  (bind _maxtime (`self.MAXTIME`))
  (bind _output_get (set `self.CurrentTime` (+ DeltaSeconds (`self.CurrentTime`))))
  (if (> _output_get _maxtime)
    (set `self.CurrentTime` (- (`self.CurrentTime`) _maxtime))
    (`self.SpawnPart`)))

(fn `SpawnPart`
  (bind _returnvalue (enumliteral `/Game/Toys/Parts` (cast `/Game/Toys/Parts` (`KismetMathLibrary.Conv_IntToByte` (`KismetMathLibrary.RandomIntegerInRange` 1 (- (`KismetMathLibrary.Conv_ByteToInt` (enumliteral `/Game/Toys/Parts` "NewEnumerator6")) 1))))))
  (if (`self.Spawn`)
    (bind _asgm_fun_factory (cast `/Game/Toys/GM_FunFactory` (`GameplayStatics.GetGameMode`)))
    (bind _returnvalue_2 (enumliteral `/Game/Toys/ToyType` (cast `/Game/Toys/ToyType` (`KismetMathLibrary.Conv_IntToByte` (`KismetMathLibrary.RandomIntegerInRange` 0 (`/Game/Toys/GM_FunFactory.DifficultyLevel` _asgm_fun_factory))))))
    (bind _returnvalue_3 (`|SpawnActorFromClass` "/Game/Toys/BP_ToyMember.BP_ToyMember_C" (`KismetMathLibrary.MakeTransform` (`KismetSystemLibrary.GetComponentBounds` (`self.Box`)) (`KismetMathLibrary.MakeRotator` 0.0 0.0 (`KismetMathLibrary.RandomFloatInRange` 0.0 360.0)) (1.0 1.0 1.0)) "AlwaysSpawn" "OverrideRootScale" null _returnvalue_2 _returnvalue))
    (bind _asgm_fun_factory_2 (cast `/Game/Toys/GM_FunFactory` (`GameplayStatics.GetGameMode`)))
    (bind _outmesh (`/Game/Toys/GM_FunFactory.ObtainMesh` _asgm_fun_factory_2 _returnvalue _returnvalue_2))
    (if (`KismetSystemLibrary.IsValid` _returnvalue_3)
      (`/Game/Toys/BP_ToyMember.Init` _returnvalue_3 _outmesh))))

(fn `UserConstructionScript`)