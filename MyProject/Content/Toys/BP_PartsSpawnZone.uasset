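; Spawn zone that periodically drops random toy parts into the Fun Factory game.
; A Tick timer calls SpawnPart each time it passes MAXTIME, spawning a BP_ToyMember at a random point in the Box bounds with random yaw, toy type and part.
; GM_FunFactory supplies the mesh passed to the part's Init, from type and part random expressions evaluated separately from the spawn's, so the two can differ.
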(event `self.ReceiveBeginPlay`)

(event `self.ReceiveActorBeginOverlap`
  (params (OtherActor :type "Actor Object Reference")))

(event `self.ReceiveTick`
  (params (DeltaSeconds :type "Float (single-precision)"))
  (bind _maxtime (`self.MAXTIME`))
  (bind _output_get (set `self.CurrentTime` (+ DeltaSeconds (`self.CurrentTime`))))
  (if (> _output_get _maxtime)
    (set `self.CurrentTime` (- (`self.CurrentTime`) _maxtime))
    (`self.SpawnPart`)))

(fn `SpawnPart`
  (bind (_origin _boxextent) (`KismetSystemLibrary.GetComponentBounds` (`self.Box`)))
  (bind _returnvalue (enumliteral `/Game/Toys/ToyType` (cast `/Game/Toys/ToyType` (`KismetMathLibrary.Conv_IntToByte` (`KismetMathLibrary.RandomIntegerInRange` 0 (- (`KismetMathLibrary.Conv_ByteToInt` (enumliteral `/Game/Toys/ToyType` "NewEnumerator1")) 1))))))
  (bind _returnvalue_2 (enumliteral `/Game/Toys/Parts` (cast `/Game/Toys/Parts` (`KismetMathLibrary.Conv_IntToByte` (`KismetMathLibrary.RandomIntegerInRange` 1 (- (`KismetMathLibrary.Conv_ByteToInt` (enumliteral `/Game/Toys/Parts` "NewEnumerator6")) 1))))))
  (bind _returnvalue_3 (`|SpawnActorFromClass` "/Game/Toys/BP_ToyMember.BP_ToyMember_C" (`KismetMathLibrary.MakeTransform` (`KismetMathLibrary.RandomPointInBoundingBox` _origin _boxextent) (`KismetMathLibrary.MakeRotator` 0.0 0.0 (`KismetMathLibrary.RandomFloatInRange` 0.0 360.0)) (1.0 1.0 1.0)) "AlwaysSpawn" "OverrideRootScale" null _returnvalue _returnvalue_2))
  (bind _asgm_fun_factory (cast `/Game/Toys/GM_FunFactory` (`GameplayStatics.GetGameMode`)))
  (bind _outmesh (`/Game/Toys/GM_FunFactory.ObtainMesh` _asgm_fun_factory _returnvalue_2 _returnvalue))
  (if (`KismetSystemLibrary.IsValid` _returnvalue_3)
    (`/Game/Toys/BP_ToyMember.Init` _returnvalue_3 _outmesh)))

(fn `UserConstructionScript`)