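; Game mode for FunFactory, a timed toy-assembly round with a randomly generated target toy.
; BeginPlay rolls GoodParts, gives the existing toy core its body mesh, hooks it to a physics constraint, spawns a scaled-up, non-simulated target at BP_SpawnPlace, and adds the timer HUD.
; Tick counts down, then stores and prints the main toy's CalculateDocks score once.
; SpawnParts is an unfinished stub with an empty loop.
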(event `self.ReceiveTick`
  (params (DeltaSeconds :type "Float (single-precision)"))
  (bind _output_get (set `self.timeleft` (- (`self.timeleft`) DeltaSeconds)))
  (if (<= _output_get 0.0)
    (set `self.TimeOver` true)
    (if (not (`self.FinalScoreCalculated`))
      (bind _outactors (`GameplayStatics.GetAllActorsOfClass` "/Game/Toys/BP_ToyCore.BP_ToyCore_C"))
      (for _array_element _outactors
        (if (`/Game/Toys/BP_ToyCore.isMainToy` _array_element)
          (bind _finalscore (`/Game/Toys/BP_ToyCore.CalculateDocks` _array_element))
          (bind _output_get_2 (set `self.FinalScore` _finalscore))
          (`KismetSystemLibrary.PrintString` (`KismetStringLibrary.Conv_IntToString` _output_get_2))
          (set `self.FinalScoreCalculated` true))))
    (else
      (set `self.TimeOver` false))))

(event `self.ReceiveBeginPlay`
  (bind _outactors (`GameplayStatics.GetAllActorsOfClass` "/Game/Toys/BP_ToyCore.BP_ToyCore_C"))
  (`self.GenerateTargetToy`)
  (bind _outmesh (`self.ObtainMesh` "NewEnumerator5" (`KismetArrayLibrary.Array_Get` (`self.GoodParts`))))
  (bind _item (`KismetArrayLibrary.Array_Get` _outactors))
  (`/Game/Toys/BP_ToyCore.Init` _item _outmesh)
  (bind _outactors_2 (`GameplayStatics.GetAllActorsOfClass` "/Script/Engine.PhysicsConstraintActor"))
  (`self.SpawnTargetToy`)
  (`PhysicsConstraintComponent.SetConstrainedComponents` (`PhysicsConstraintActor.ConstraintComp` (`KismetArrayLibrary.Array_Get` _outactors_2)) (`/Game/Toys/BP_ToyCore.Mesh` _item) "None" null "None")
  (bind _returnvalue (`|CreateWidget` "/Game/Level/TimerHUD.TimerHUD_C"))
  (`UserWidget.AddToViewport` _returnvalue 0))

(fn `GenerateTargetToy`
  (for _index (range 7)
    (`KismetArrayLibrary.Array_Set` (`self.GoodParts`) _index (cast `/Game/Toys/ToyType` (`KismetMathLibrary.Conv_IntToByte` (`KismetMathLibrary.RandomIntegerInRange` 0 (- (`KismetMathLibrary.Conv_ByteToInt` (enumliteral `/Game/Toys/ToyType` "NewEnumerator1")) 1)))))))

(fn `ObtainMesh`
  (params (inPart :type "/Game/Toys/Parts Enum") (inType :type "/Game/Toys/ToyType Enum"))
  (returns (outMesh :type "StaticMesh Object Reference"))
  (bind (_body _head _armleft _armright _legleft _legright) (break `/Game/Toys/ToyStruct` (`KismetArrayLibrary.Array_Get` (`self.AllMeshes`) (`KismetMathLibrary.Conv_ByteToInt` inType))))
  (return (select `int` (`KismetMathLibrary.Conv_ByteToInt` inPart) :`0` _body :`1` _head :`2` _armleft :`3` _armright :`4` _legleft :`5` _legright)))

(fn `SpawnParts`
  (bind _outactors (`GameplayStatics.GetAllActorsOfClass` "/Game/Toys/BP_PartsSpawnZone.BP_PartsSpawnZone_C"))
  (for _ _outactors
    _))

(fn `SpawnTargetToy`
  (bind _outactors (`GameplayStatics.GetAllActorsOfClass` "/Game/Toys/BP_SpawnPlace.BP_SpawnPlace_C"))
  (bind _returnvalue (`|SpawnActorFromClass` "/Game/Toys/BP_ToyCore.BP_ToyCore_C" (`KismetMathLibrary.MakeTransform` (.location (`SceneComponent.K2_GetComponentToWorld` (`/Game/Toys/BP_SpawnPlace.DefaultSceneRoot` (`KismetArrayLibrary.Array_Get` _outactors)))) (.rotation (`SceneComponent.K2_GetComponentToWorld` (`/Game/Toys/BP_SpawnPlace.DefaultSceneRoot` (`KismetArrayLibrary.Array_Get` _outactors)))) (15.0 15.0 15.0)) "AlwaysSpawn" "OverrideRootScale"))
  (set `/Game/Toys/BP_ToyCore.isMainToy` false _returnvalue)
  (`PrimitiveComponent.SetSimulatePhysics` (`/Game/Toys/BP_ToyCore.Mesh` _returnvalue) false)
  (bind _outmesh (`self.ObtainMesh` "NewEnumerator5" (`KismetArrayLibrary.Array_Get` (`self.GoodParts`))))
  (`/Game/Toys/BP_ToyCore.Init` _returnvalue _outmesh)
  (for _index (range 1 6)
    (bind _item (`KismetArrayLibrary.Array_Get` (`self.GoodParts`) _index))
    (bind _returnvalue_2 (enumliteral `/Game/Toys/Parts` (cast `/Game/Toys/Parts` (`KismetMathLibrary.Conv_IntToByte` _index))))
    (bind _returnvalue_3 (`|SpawnActorFromClass` "/Game/Toys/BP_ToyMember.BP_ToyMember_C" (`SceneComponent.K2_GetComponentToWorld` (select `int` (- _index 1) :`0` (`/Game/Toys/BP_ToyCore.Head` _returnvalue) :`1` (`/Game/Toys/BP_ToyCore.Arm_Left` _returnvalue) :`2` (`/Game/Toys/BP_ToyCore.Arm_Right` _returnvalue) :`3` (`/Game/Toys/BP_ToyCore.Leg_Left` _returnvalue) :`4` (`/Game/Toys/BP_ToyCore.Leg_Right` _returnvalue))) "AlwaysSpawn" "OverrideRootScale" null _item _returnvalue_2))
    (`PrimitiveComponent.SetSimulatePhysics` (`/Game/Toys/BP_ToyMember.Mesh` _returnvalue_3) false)
    (bind _outmesh_2 (`self.ObtainMesh` _returnvalue_2 _item))
    (`/Game/Toys/BP_ToyMember.Init` _returnvalue_3 _outmesh_2)
    (`self.K2_AttachRootComponentTo` (`/Game/Toys/BP_ToyCore.Mesh` _returnvalue))))

(fn `UserConstructionScript`)