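; Central body of a toy that collects BP_ToyMember parts and scores how well it is assembled, showing its rope only on the main toy.
; Parts that hit the mesh attach where they touch with a spark effect and join MemberList.
; CalculateDocks totals five head, arm and leg docks, scoring members inside each dock's sphere radius on correct position and on type matching GM_FunFactory's GoodParts.
; Init sets the body mesh.
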(event OnComponentHit(Mesh)
  (params (OtherActor :type Actor%20Object%20Reference) (OtherComp :type Primitive%20Component%20Object%20Reference) (NormalImpulse :type Vector :default "0, 0, 0") (Hit :type Hit%20Result%20Structure%20%28by%20ref%29))
  (bind (_bblockinghit _binitialoverlap _time _location _impactpoint _normal _impactnormal) (Collision|BreakHitResult Hit))
  (bind _asbp_toy_member (Utilities|Casting|CastToBP_ToyMember OtherActor))
  (if (not (Utilities|Array|ContainsItem (Variables|Default|GetMemberList) _asbp_toy_member))
    (Class|Actor|AttachRootComponentto _asbp_toy_member (Variables|Default|GetMesh) "None" "KeepWorldPosition" true)
    (Utilities|Array|Add (Variables|Default|GetMemberList) _asbp_toy_member)
    (Variables|/Game/Toys/BP_ToyMember.BP_ToyMember_C|SetattachedToCore _asbp_toy_member true)
    (Effects|SpawnEmitterAttached "/Game/StarterContent/Particles/P_Sparks.P_Sparks" (Variables|Default|GetMesh) "None" _location (Math|Vector|RotatorfromAxisandAngle _normal (Math|Vector|DotProduct _normal _impactnormal)) "KeepWorldPosition")))

(event EventBeginPlay
  (bind _bp_rope (Variables|Default|GetBP_Rope))
  (if (Variables|Default|GetisMainToy)
    (Rendering|SetVisibility _bp_rope true true)
    (else
      (Rendering|SetVisibility _bp_rope false true))))

(event EventActorBeginOverlap
  (params (OtherActor :type Actor%20Object%20Reference)))

(event EventTick
  (params (DeltaSeconds :type Float%20%28single-precision%29)))

(fn ConstructionScript)

(fn CalculateDocks
  (bind _scoreout (CallFunction|CalculateDock "NewEnumerator2" (Variables|Default|GetArm_Right)))
  (Variables|Default|SetScoreTotal (+ _scoreout (Variables|Default|GetScoreTotal)))
  (bind _scoreout_2 (CallFunction|CalculateDock "NewEnumerator1" (Variables|Default|GetArm_Left)))
  (Variables|Default|SetScoreTotal (+ _scoreout_2 (Variables|Default|GetScoreTotal)))
  (bind _scoreout_3 (CallFunction|CalculateDock "NewEnumerator0" (Variables|Default|GetHead)))
  (Variables|Default|SetScoreTotal (+ _scoreout_3 (Variables|Default|GetScoreTotal)))
  (bind _scoreout_4 (CallFunction|CalculateDock "NewEnumerator3" (Variables|Default|GetLeg_Left)))
  (Variables|Default|SetScoreTotal (+ _scoreout_4 (Variables|Default|GetScoreTotal)))
  (bind _scoreout_5 (CallFunction|CalculateDock "NewEnumerator4" (Variables|Default|GetLeg_Right)))
  (bind _output_get (Variables|Default|SetScoreTotal (+ _scoreout_5 (Variables|Default|GetScoreTotal))))
  (return _output_get))

(fn CalculateDock
  (params (Position :type Parts%20Enum) (PartCollision :type Sphere%20Component%20Object%20Reference))
  (bind _asgm_fun_factory (Utilities|Casting|CastToGM_FunFactory (Game|GetGameMode))
    (:then
      (for _array_element (Variables|Default|GetMemberList)
        (if (> (Components|Sphere|GetScaledSphereRadius PartCollision) (Math|Vector|VectorLength (- (Transformation|GetWorldLocation (Variables|/Game/Toys/BP_ToyMember.BP_ToyMember_C|Getcollision _array_element)) (Transformation|GetWorldLocation PartCollision))))
          (if (Utilities|Enum|Equal(Enum) (Variables|/Game/Toys/BP_ToyMember.BP_ToyMember_C|Getpart _array_element) Position)
            (LocalVariables|SetScore (+ (LocalVariables|GetScore) 50)))
          (if (Utilities|Enum|Equal(Enum) (Variables|/Game/Toys/BP_ToyMember.BP_ToyMember_C|Gettype _array_element) (Utilities|Array|Get(acopy) (Variables|/Game/Toys/GM_FunFactory.GM_FunFactory_C|GetGoodParts _asgm_fun_factory) (Math|Conversions|ToInteger(Byte) (Variables|/Game/Toys/BP_ToyMember.BP_ToyMember_C|Getpart _array_element))))
            (LocalVariables|SetScore (+ (LocalVariables|GetScore) 50)))
          (if (> (LocalVariables|GetScore) (LocalVariables|GetScoreMax))
            (LocalVariables|SetScoreMax (LocalVariables|GetScore))
            (LocalVariables|SetScore 0))))
      (return (LocalVariables|GetScoreMax)))
    (:CastFailed
      (return 0))))

(fn Init
  (params (InMesh :type Static%20Mesh%20Object%20Reference))
  (Components|StaticMesh|SetStaticMesh (Variables|Default|GetMesh) InMesh))