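; Objective platform actor that lets the player toggle a Matinee sequence forward and backward with the space bar.
; On BeginPlay it enables input from player controller 0.
; Each Space press flips a Toggle flag, then plays or reverses the first MatineeActor found in the level through GetAllActorsOfClass, rather than a specific reference.
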(event `Key|SpaceBar`
  (params (Key :type "Key Structure" :default "AnyKey"))
  (:`Pressed`
    (bind _outactors (`GameplayStatics.GetAllActorsOfClass` "/Script/Engine.MatineeActor"))
    (bind _output_get (set `self.toggle` (not (`self.toggle`))))
    (if _output_get
      (bind _item (`KismetArrayLibrary.Array_Get` _outactors))
      (`MatineeActor.Play` _item)
      (else
        (`MatineeActor.Reverse` _item)))))

(event `self.ReceiveBeginPlay`
  (`self.EnableInput` (`GameplayStatics.GetPlayerController` 0)))

(event `self.ReceiveActorBeginOverlap`
  (params (OtherActor :type "Actor Object Reference")))

(event `self.ReceiveTick`
  (params (DeltaSeconds :type "Float (single-precision)")))

(fn `UserConstructionScript`)