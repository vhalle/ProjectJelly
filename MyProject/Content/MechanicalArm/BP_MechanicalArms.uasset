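; Player-possessed pawn with two gamepad-driven mechanical arms that pick up toy parts, one arm controlled at a time.
; The top face button swaps the current pivot and pedestal references and flips rotation direction.
; Stick input rotates the clamped elbow and shoulder at dead-zoned, two-tier speeds, while triggers slide the pedestal on Tick.
; Each hand attaches an overlapping BP_ToyMember to its wrist until Tick detects it attached to the core.
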(event OnComponentBeginOverlap(LHandCollisions)
  (params (OtherActor :type Actor%20Object%20Reference) (OtherComp :type Primitive%20Component%20Object%20Reference) (OtherBodyIndex :type Integer) (bFromSweep :type Boolean) (SweepResult :type Hit%20Result%20Structure%20%28by%20ref%29))
  (if (not (Variables|Default|GetLattachedToAToy))
    (bind _asbp_toy_member (Utilities|Casting|CastToBP_ToyMember OtherActor))
    (if (not (Variables|/Game/Toys/BP_ToyMember.BP_ToyMember_C|GetattachedToCore _asbp_toy_member))
      (Class|Actor|AttachRootComponentto _asbp_toy_member (Variables|Default|GetLWristPivot) "None" "KeepWorldPosition" true)
      (Variables|Default|SetLcurrentToy _asbp_toy_member)
      (Variables|Default|SetLattachedToAToy true)
      (Variables|/Game/Toys/BP_ToyMember.BP_ToyMember_C|SetattachedToArm (Variables|Default|GetLcurrentToy) true))))

(event OnComponentBeginOverlap(RHandCollisions)
  (params (OtherActor :type Actor%20Object%20Reference) (OtherComp :type Primitive%20Component%20Object%20Reference) (OtherBodyIndex :type Integer) (bFromSweep :type Boolean) (SweepResult :type Hit%20Result%20Structure%20%28by%20ref%29))
  (if (not (Variables|Default|GetRAttachedToAToy))
    (bind _asbp_toy_member (Utilities|Casting|CastToBP_ToyMember OtherActor))
    (if (not (Variables|/Game/Toys/BP_ToyMember.BP_ToyMember_C|GetattachedToCore _asbp_toy_member))
      (Class|Actor|AttachRootComponentto _asbp_toy_member (Variables|Default|GetRWristPivot) "None" "KeepWorldPosition" true)
      (Variables|Default|SetRcurrentToy _asbp_toy_member)
      (Variables|Default|SetRAttachedToAToy true)
      (Variables|/Game/Toys/BP_ToyMember.BP_ToyMember_C|SetattachedToArm (Variables|Default|GetRcurrentToy) true))))

(event EventBeginPlay
  (Pawn|Possess (Game|GetPlayerController 0) self)
  (Variables|Default|SetcurrentShoulderPivot (Variables|Default|GetRShoulderPivot))
  (Variables|Default|SetcurrentElbowPivot (Variables|Default|GetRElbowPivot))
  (Variables|Default|SetcurrentPedestal (Variables|Default|GetRPedestal))
  (Variables|Default|SetcurrentHandCollisionSphere (Variables|Default|GetRHandCollisions))
  (Variables|Default|SetrotationMultiplicator -1))

(event EventTick
  (params (DeltaSeconds :type Float%20%28single-precision%29))
  (bind _currentpedestal (Variables|Default|GetcurrentPedestal))
  (bind _currentpedestal_2 (Variables|Default|GetcurrentPedestal))
  (bind _relativelocation (Variables|/Script/Engine.SceneComponent|GetRelativeLocation _currentpedestal))
  (bind _relativelocation_2 (Variables|/Script/Engine.SceneComponent|GetRelativeLocation _currentpedestal_2))
  (bind (_x _y _z) (Math|Vector|BreakVector _relativelocation))
  (bind (_x_2 _y_2 _z_2) (Math|Vector|BreakVector _relativelocation_2))
  (CallFunction|VerifyToysAttachment)
  (if (== (Class|PlayerController|GetInputAnalogKeyState (Game|GetPlayerController 0) "Gamepad_LeftTrigger") 1.0)
    (bind _newparam (CallFunction|SetFloatinRange -3e+02 3e+02 (+ _x_2 6.0)))
    (Transformation|SetRelativeLocation _currentpedestal_2 (Math|Vector|MakeVector _newparam _y_2 _z_2) false false))
  (if (== (Class|PlayerController|GetInputAnalogKeyState (Game|GetPlayerController 0) "Gamepad_RightTrigger") 1.0)
    (bind _newparam_2 (CallFunction|SetFloatinRange -3e+02 3e+02 (- _x 6.0)))
    (Transformation|SetRelativeLocation _currentpedestal (Math|Vector|MakeVector _newparam_2 _y _z) false false)))

(event Input|GamepadEvents|GamepadLeftX
  (params (AxisValue :type Float%20%28single-precision%29))
  (bind _currentelbowpivot (Variables|Default|GetcurrentElbowPivot))
  (bind _relativerotation (Variables|/Script/Engine.SceneComponent|GetRelativeRotation _currentelbowpivot))
  (bind (_roll _pitch _yaw) (Math|Rotator|BreakRotator _relativerotation))
  (bind _rotationspeed (CallFunction|GetRotationSpeed AxisValue))
  (bind _newparam (CallFunction|SetFloatinRange 1e+01 1.4e+02 (+ _roll _rotationspeed)))
  (Transformation|SetRelativeRotation (Variables|Default|GetcurrentElbowPivot) (Math|Rotator|MakeRotator _newparam _pitch _yaw) false false))

(event Input|GamepadEvents|GamepadLeftY
  (params (AxisValue :type Float%20%28single-precision%29))
  (bind _currentshoulderpivot (Variables|Default|GetcurrentShoulderPivot))
  (bind _relativerotation (Variables|/Script/Engine.SceneComponent|GetRelativeRotation _currentshoulderpivot))
  (bind (_roll _pitch _yaw) (Math|Rotator|BreakRotator _relativerotation))
  (bind _rotationspeed (CallFunction|GetRotationSpeed AxisValue))
  (if (Variables|Default|GetcontrolLeftArm)
    (bind _newparam (CallFunction|SetFloatinRange -4e+01 3e+01 (+ _rotationspeed _roll)))
    (Transformation|SetRelativeRotation (Variables|Default|GetcurrentShoulderPivot) (Math|Rotator|MakeRotator _newparam _pitch _yaw) false false)
    (else
      (bind _newparam_2 (CallFunction|SetFloatinRange -3e+01 4e+01 (+ _rotationspeed _roll)))
      (Transformation|SetRelativeRotation (Variables|Default|GetcurrentShoulderPivot) (Math|Rotator|MakeRotator _newparam_2 _pitch _yaw) false false))))

(event Input|GamepadEvents|GamepadRightX
  (params (AxisValue :type Float%20%28single-precision%29)))

(event Input|GamepadEvents|GamepadRightY
  (params (AxisValue :type Float%20%28single-precision%29)))

(event Input|GamepadEvents|GamepadFaceButtonTop
  (params (Key :type Key%20Structure :default "AnyKey"))
  (:Pressed
    (CallFunction|ChangeArm)))

(fn ConstructionScript)

(fn GetRotationSpeed
  (params (axisValue :type Float%20%28single-precision%29))
  (LocalVariables|SetaxisValue_ axisValue)
  (if (or (>= (LocalVariables|GetaxisValue_) 0.7) (<= (LocalVariables|GetaxisValue_) -0.7))
    (return (* (LocalVariables|GetaxisValue_) (Variables|Default|GetmaxRotationSpeed) (Math|Conversions|ToFloat(Integer) (Variables|Default|GetrotationMultiplicator))))
    (elif (or (>= (LocalVariables|GetaxisValue_) 0.3) (<= (LocalVariables|GetaxisValue_) -0.3))
      (return (* (Variables|Default|GetminRotationSpeed) (LocalVariables|GetaxisValue_) (Math|Conversions|ToFloat(Integer) (Variables|Default|GetrotationMultiplicator))))
      (else
        (return 0.0)))))

(fn SetFloatinRange
  (params (min :type Float%20%28single-precision%29) (max :type Float%20%28single-precision%29) (value :type Float%20%28single-precision%29))
  (if (> value max)
    (return max)
    (elif (< value min)
      (return min)
      (else
        (return value)))))

(fn ChangeArm
  (bind _output_get (Variables|Default|SetcontrolLeftArm (not (Variables|Default|GetcontrolLeftArm))))
  (if _output_get
    (Variables|Default|SetcurrentShoulderPivot (Variables|Default|GetLShoulderPivot))
    (Variables|Default|SetcurrentElbowPivot (Variables|Default|GetLElbowPivot))
    (Variables|Default|SetcurrentPedestal (Variables|Default|GetLPedestal))
    (Variables|Default|SetcurrentHandCollisionSphere (Variables|Default|GetLHandCollisions))
    (Variables|Default|SetrotationMultiplicator 1)
    (else
      (Variables|Default|SetcurrentShoulderPivot (Variables|Default|GetRShoulderPivot))
      (Variables|Default|SetcurrentElbowPivot (Variables|Default|GetRElbowPivot))
      (Variables|Default|SetcurrentPedestal (Variables|Default|GetRPedestal))
      (Variables|Default|SetcurrentHandCollisionSphere (Variables|Default|GetRHandCollisions))
      (Variables|Default|SetrotationMultiplicator -1))))

(fn VerifyToysAttachment
  (bind _lcurrenttoy (Variables|Default|GetLcurrentToy))
  (bind _rcurrenttoy (Variables|Default|GetRcurrentToy))
  (Utilities|IsValid (Variables|Default|GetLcurrentToy)
    (:Is%20Valid
      (if (Variables|/Game/Toys/BP_ToyMember.BP_ToyMember_C|GetattachedToCore _lcurrenttoy)
        (Variables|/Game/Toys/BP_ToyMember.BP_ToyMember_C|SetattachedToArm _lcurrenttoy false)
        (Variables|Default|SetLattachedToAToy false)))
    (:Is%20Not%20Valid
      _))
  (Utilities|IsValid (Variables|Default|GetRcurrentToy)
    (:Is%20Valid
      (if (Variables|/Game/Toys/BP_ToyMember.BP_ToyMember_C|GetattachedToCore _rcurrenttoy)
        (Variables|/Game/Toys/BP_ToyMember.BP_ToyMember_C|SetattachedToArm _rcurrenttoy false)
        (Variables|Default|SetRAttachedToAToy false)))))