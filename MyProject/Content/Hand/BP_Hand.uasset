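; BP_Hand is a three-fingered hand that animates opening and closing by rotating the middle pivots of its fingers.
; CloseHand and OpenHand set request flags, which Tick reads to call SetMiddleFingerRotation each frame.
; That function steps the shared finger 1/3 pivot and the finger 2 pivot in opposite roll directions, clamped to fixed ranges.
; Finger 2 reaching its limit clears the request and updates the open, closed and moving states.
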(event EventTick
  (params (DeltaSeconds :type Float%20%28single-precision%29))
  (if (and (Variables|Default|GetmustClose) (not (Variables|Default|GetisClosed)))
    (Variables|Default|SetisMoving true)
    (CallFunction|SetMiddleFingerRotation true)
    (Variables|Default|SetisOpen false)
    (Utilities|FlowControl|Delay 0.2 :!label _label)
    (elif (and (Variables|Default|GetmustOpen) (not (Variables|Default|GetisOpen)))
      (Variables|Default|SetisMoving true)
      (CallFunction|SetMiddleFingerRotation false)
      (Variables|Default|SetisClosed false)
      (goto _label))))

(fn ConstructionScript)

(fn SetMiddleFingerRotation
  (params (closing :type Boolean))
  (bind _finger1and3middlepivot (Variables|Default|GetFinger1And3MiddlePivot))
  (bind _finger2middlepivot (Variables|Default|GetFinger2MiddlePivot))
  (bind _const_delta_angle (LocalVariables|GetCONST_DELTA_ANGLE))
  (bind _relativerotation (Variables|/Script/Engine.SceneComponent|GetRelativeRotation _finger2middlepivot))
  (bind _relativerotation_2 (Variables|/Script/Engine.SceneComponent|GetRelativeRotation _finger1and3middlepivot))
  (bind (_roll _pitch _yaw) (Math|Rotator|BreakRotator _relativerotation))
  (bind (_roll_2 _pitch_2 _yaw_2) (Math|Rotator|BreakRotator _relativerotation_2))
  (if closing
    (LocalVariables|SetdeltaAngle _const_delta_angle)
    (else
      (LocalVariables|SetdeltaAngle (* -1 _const_delta_angle))))
  (bind _newparam (CallFunction|SetFloatinRange -55.0 -1e+01 (+ (LocalVariables|GetdeltaAngle) _roll_2)))
  (Transformation|SetRelativeRotation (Variables|Default|GetFinger1And3MiddlePivot) (Math|Rotator|MakeRotator _newparam _pitch_2 _yaw_2) false false)
  (bind _newparam_2 (CallFunction|SetFloatinRange 6.0 51.0 (- _roll (LocalVariables|GetdeltaAngle))))
  (if (and (Variables|Default|GetmustClose) (== _newparam_2 6.0))
    (Variables|Default|SetmustClose false)
    (Variables|Default|SetisClosed true)
    (Variables|Default|SetisMoving false :!label _label)
    (elif (and (Variables|Default|GetmustOpen) (== _newparam_2 51.0))
      (Variables|Default|SetmustOpen false)
      (Variables|Default|SetisOpen true)
      (goto _label)
      (else
        _)))
  (Transformation|SetRelativeRotation (Variables|Default|GetFinger2MiddlePivot) (Math|Rotator|MakeRotator _newparam_2 _pitch _yaw) false false))

(fn CloseHand
  (Variables|Default|SetmustClose true))

(fn OpenHand
  (Variables|Default|SetmustOpen true))

(fn SetFloatinRange
  (params (min :type Float%20%28single-precision%29) (max :type Float%20%28single-precision%29) (value :type Float%20%28single-precision%29))
  (if (> value max)
    (return max)
    (elif (< value min)
      (return min)
      (else
        (return value)))))